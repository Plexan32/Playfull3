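; BP_Paint2 is an interactable paint object in level 1 that tracks a painting puzzle through the player Blueprint.
; DoorInteract increments the player's PaintIndex and swaps the static mesh to its colored horse variant.
; Tick polls the player, reverting to the empty mesh once per Lose state and destroying the actor when the player's True flag is set.
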(event `self.ReceiveBeginPlay`
  (bind _asbp_player (cast `/Game/Ramko/Lvl1/BP_Player` (`GameplayStatics.GetPlayerCharacter` 0)))
  (set `self.As BP Player` _asbp_player))

(event `/Game/Ramko/General/BI_DoorInteraction.DoorInteract`
  (bind _as_bp_player (`self.As BP Player`))
  (bind _result (`/Engine/EditorBlueprintResources/StandardMacros.IncrementInt` (`/Game/Ramko/Lvl1/BP_Player.PaintIndex` _as_bp_player))
    (:`  `
      (set `/Game/Ramko/Lvl1/BP_Player.PaintIndex` _result _as_bp_player)
      (`StaticMeshComponent.SetStaticMesh` (`self.StaticMesh`) "/Game/Ramko/Lvl1/Cocuk_cizim/Dolu_resimler/Mesh_At_renkli.Mesh_At_renkli"))))

(event `self.ReceiveTick`
  (params (DeltaSeconds :type "Float (single-precision)"))
  (`|ExecutionSequence`
    (:`then_0`
      (if (`/Game/Ramko/Lvl1/BP_Player.Lose?` (`self.As BP Player`))
        (`/Engine/EditorBlueprintResources/StandardMacros.DoOnce` false :!label _label
          (:`Completed`
            (`StaticMeshComponent.SetStaticMesh` (`self.StaticMesh`) "/Game/Ramko/Lvl1/Cocuk_cizim/Bos_resimler/Mesh_At_Bos.Mesh_At_Bos")))
        (else
          (goto _label :!via `Reset`))))
    (:`then_1`
      (if (`/Game/Ramko/Lvl1/BP_Player.True?` (`self.As BP Player`))
        (`self.K2_DestroyActor`)))))

(fn `UserConstructionScript`)