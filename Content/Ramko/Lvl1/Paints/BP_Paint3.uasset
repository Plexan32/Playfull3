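; BP_Paint3 is an interactable level 1 paint actor that updates the player's PaintIndex counter.
; It caches BP_Player at BeginPlay and uses a Box overlap to allow interaction only while the player is inside.
; On DoorInteract, it increments PaintIndex and then immediately sets it to 0, so the counter always ends reset.
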(event `self.ReceiveBeginPlay`
  (bind _asbp_player (cast `/Game/Ramko/Lvl1/BP_Player` (`GameplayStatics.GetPlayerCharacter` 0)))
  (set `self.As BP Player` _asbp_player))

(event `/Game/Ramko/General/BI_DoorInteraction.DoorInteract`
  (bind _as_bp_player (`self.As BP Player`))
  (if (`self.CanInteract`)
    (`/Engine/EditorBlueprintResources/StandardMacros.IncrementInt` (`/Game/Ramko/Lvl1/BP_Player.PaintIndex` _as_bp_player)
      (:`  `
        (set `/Game/Ramko/Lvl1/BP_Player.PaintIndex` 0 _as_bp_player)))))

(event `self.Box.OnComponentBeginOverlap`
  (params (OverlappedComponent :type "PrimitiveComponent Object Reference") (OtherActor :type "Actor Object Reference") (OtherComp :type "PrimitiveComponent Object Reference") (OtherBodyIndex :type Integer) (bFromSweep :type Boolean) (SweepResult :type "HitResult Structure (by ref)"))
  (cast `/Game/Ramko/Lvl1/BP_Player` OtherActor)
  (set `self.CanInteract` true))

(event `self.Box.OnComponentEndOverlap`
  (params (OverlappedComponent :type "PrimitiveComponent Object Reference") (OtherActor :type "Actor Object Reference") (OtherComp :type "PrimitiveComponent Object Reference") (OtherBodyIndex :type Integer))
  (cast `/Game/Ramko/Lvl1/BP_Player` OtherActor)
  (set `self.CanInteract` false))

(fn `UserConstructionScript`)