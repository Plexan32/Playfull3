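; BP_EndDoor3 is a Level 3 door actor that swings open when interacted with while the player is in range.
; Box overlaps with BP_Player3 toggle CanInteract, which gates the DoorInteract event.
; DoorInteract plays a timeline that lerps actor yaw toward an absolute angle, blending from the current rotation each update rather than a stored start.
; BeginPlay caches a player reference that these graphs never use.
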(event `self.ReceiveBeginPlay`
  (bind _asbp_player_3 (cast `/Game/Ramko/Lvl3/BP_Player3` (`GameplayStatics.GetPlayerCharacter` 0)))
  (set `self.As BP Player 3` _asbp_player_3))

(event `/Game/Ramko/General/BI_DoorInteraction.DoorInteract`
  (bind (_returnvalue_roll _returnvalue_pitch) (`KismetMathLibrary.BreakRotator` (`self.K2_GetActorRotation`)))
  (if (`self.CanInteract?`)
    (bind (_direction _newtrack_0) (`Timeline|Timeline` :!via `PlayFromStart`)
      (:`Update`
        (`self.K2_SetActorRotation` (`KismetMathLibrary.RLerp` (`self.K2_GetActorRotation`) (`KismetMathLibrary.MakeRotator` _returnvalue_roll _returnvalue_pitch -90.0) _newtrack_0))))))

(event `self.Box.OnComponentBeginOverlap`
  (params (OverlappedComponent :type "PrimitiveComponent Object Reference") (OtherActor :type "Actor Object Reference") (OtherComp :type "PrimitiveComponent Object Reference") (OtherBodyIndex :type Integer) (bFromSweep :type Boolean) (SweepResult :type "HitResult Structure (by ref)"))
  (cast `/Game/Ramko/Lvl3/BP_Player3` OtherActor)
  (set `self.CanInteract?` true))

(event `self.Box.OnComponentEndOverlap`
  (params (OverlappedComponent :type "PrimitiveComponent Object Reference") (OtherActor :type "Actor Object Reference") (OtherComp :type "PrimitiveComponent Object Reference") (OtherBodyIndex :type Integer))
  (cast `/Game/Ramko/Lvl3/BP_Player3` OtherActor)
  (set `self.CanInteract?` false))

(fn `UserConstructionScript`)