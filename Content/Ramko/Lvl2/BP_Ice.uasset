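; BP_Ice is a breakable ice actor in Lvl2 that shatters when struck by a BP_Laser actor.
; On BeginPlay it caches a reference to the BP_Player2 character.
; A laser hit plays one of two random glass-breaking sounds, increments the player's Index counter, then destroys the ice.
; The sound's location is converted from that Index value rather than taken from the ice's position.
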(event `self.ReceiveBeginPlay`
  (bind _asbp_player_2 (cast `/Game/Ramko/Lvl2/BP_Player2` (`GameplayStatics.GetPlayerCharacter` 0)))
  (set `self.As BP Player 2` _asbp_player_2))

(event `self.ReceiveHit`
  (params (MyComp :type "PrimitiveComponent Object Reference") (Other :type "Actor Object Reference") (OtherComp :type "PrimitiveComponent Object Reference") (bSelfMoved :type Boolean) (HitLocation :type "Vector Structure") (HitNormal :type "Vector Structure") (NormalImpulse :type "Vector Structure") (Hit :type "HitResult Structure (by ref)"))
  (bind _index (`/Game/Ramko/Lvl2/BP_Player2.Index` (`self.As BP Player 2`)))
  (cast `/Game/Ramko/Lvl2/BP_Laser` Other)
  (`GameplayStatics.PlaySoundAtLocation` (`|GetArrayItem` (`self.CamKırılma`) (`KismetMathLibrary.RandomIntegerInRange` 0 1)) (`KismetMathLibrary.Conv_IntToVector` _index) (struct) 1.0 1.0 0.0 null null null null)
  (`/Engine/EditorBlueprintResources/StandardMacros.IncrementInt` _index
    (:`  `
      (`self.K2_DestroyActor`))))

(fn `UserConstructionScript`)