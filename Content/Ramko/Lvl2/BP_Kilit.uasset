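; BP_Kilit is a lock-like obstacle actor in level 2 that breaks when hit by a laser.
; On BeginPlay it caches the player as BP_Player2.
; When a BP_Laser hits it while the player's Index equals 3, it destroys itself and sets the player's IsIceBroke flag.
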(event `self.ReceiveBeginPlay`
  (bind _asbp_player_2 (cast `/Game/Ramko/Lvl2/BP_Player2` (`GameplayStatics.GetPlayerCharacter` 0)))
  (set `self.As BP Player 2` _asbp_player_2))

(event `self.ReceiveHit`
  (params (MyComp :type "PrimitiveComponent Object Reference") (Other :type "Actor Object Reference") (OtherComp :type "PrimitiveComponent Object Reference") (bSelfMoved :type Boolean) (HitLocation :type "Vector Structure") (HitNormal :type "Vector Structure") (NormalImpulse :type "Vector Structure") (Hit :type "HitResult Structure (by ref)"))
  (cast `/Game/Ramko/Lvl2/BP_Laser` Other)
  (if (== (`/Game/Ramko/Lvl2/BP_Player2.Index` (`self.As BP Player 2`)) 3)
    (`self.K2_DestroyActor`)
    (set `/Game/Ramko/Lvl2/BP_Player2.IsIceBroke?` true (`self.As BP Player 2`))))

(fn `UserConstructionScript`)