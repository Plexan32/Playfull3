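; BP_EndDoor2 is an interactable double door that opens only once the player's IsIceBroke flag is set.
; An overlap box enables interaction while BP_Player2 is inside, and DoorInteract checks the flag on the player cached at BeginPlay.
; When unlocked, a timeline lerps both door meshes toward zero yaw; otherwise, a doorknob timeline nudges two child actors upward as locked feedback.
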(event `self.ReceiveBeginPlay`
  (bind _asbp_player_2 (cast `/Game/Ramko/Lvl2/BP_Player2` (`GameplayStatics.GetPlayerCharacter` 0)))
  (set `self.As BP Player 2` _asbp_player_2))

(event `/Game/Ramko/General/BI_DoorInteraction.DoorInteract`
  (bind _relativelocation (`SceneComponent.RelativeLocation` (`self.ChildActor`)))
  (bind _relativelocation_2 (`SceneComponent.RelativeLocation` (`self.ChildActor1`)))
  (if (`self.CanInteract?`)
    (if (`/Game/Ramko/Lvl2/BP_Player2.IsIceBroke?` (`self.As BP Player 2`))
      (bind (_direction _newtrack_0) (`Timeline|Timeline_0` :!via `PlayFromStart`)
        (:`Update`
          (`|ExecutionSequence`
            (:`then_0`
              (`SceneComponent.K2_SetRelativeRotation` (`self.StaticMesh1`) (`KismetMathLibrary.RLerp` (`SceneComponent.RelativeRotation` (`self.StaticMesh1`)) (`KismetMathLibrary.MakeRotator` 0.0 0.0 0.0) _newtrack_0) false false)
              (`Timeline|Timeline` :!via `PlayFromStart`))
            (:`then_1`
              (`SceneComponent.K2_SetRelativeRotation` (`self.StaticMesh`) (`KismetMathLibrary.RLerp` (`SceneComponent.RelativeRotation` (`self.StaticMesh`)) (`KismetMathLibrary.MakeRotator` 0.0 0.0 0.0) _newtrack_0) false false)))))
      (else
        ;[0 0 0] DoorKnobAnim
        (bind (_direction_2 _newtrack_0_2) (`Timeline|DoorknobAnim` :!via `PlayFromStart`)
          (:`Update`
            (`|ExecutionSequence`
              (:`then_0`
                (`SceneComponent.K2_SetRelativeLocation` (`self.ChildActor1`) (`KismetMathLibrary.VLerp` _relativelocation_2 (+ _relativelocation_2 (0.0 0.0 10.0)) _newtrack_0_2) false false))
              (:`then_1`
                (`SceneComponent.K2_SetRelativeLocation` (`self.ChildActor`) (`KismetMathLibrary.VLerp` _relativelocation (+ _relativelocation (0.0 0.0 10.0)) _newtrack_0_2) false false)))))))))

(event `self.Box.OnComponentBeginOverlap`
  (params (OverlappedComponent :type "PrimitiveComponent Object Reference") (OtherActor :type "Actor Object Reference") (OtherComp :type "PrimitiveComponent Object Reference") (OtherBodyIndex :type Integer) (bFromSweep :type Boolean) (SweepResult :type "HitResult Structure (by ref)"))
  (cast `/Game/Ramko/Lvl2/BP_Player2` OtherActor)
  (set `self.CanInteract?` true))

(event `self.Box.OnComponentEndOverlap`
  (params (OverlappedComponent :type "PrimitiveComponent Object Reference") (OtherActor :type "Actor Object Reference") (OtherComp :type "PrimitiveComponent Object Reference") (OtherBodyIndex :type Integer))
  (cast `/Game/Ramko/Lvl2/BP_Player2` OtherActor)
  (set `self.CanInteract?` false))

(fn `UserConstructionScript`)